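; Market customer NPC that walks to the market, voices a greeting and fruit request, then takes a basket and leaves.
; Tick and PickupBox overlaps drive come, pickup and negative states, waiting for dialog audio to finish.
; An overlapping BasketBP is checked against the wanted fruit counts; once the externally set pickup state arrives, it attaches to her hand socket.
; Dialog sounds load by asset path from data table rows.
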(event OnComponentBeginOverlap(PickupBox)
  (params (OverlappedComponent :type Primitive%20Component%20Object%20Reference) (OtherActor :type Actor%20Object%20Reference) (OtherComp :type Primitive%20Component%20Object%20Reference) (OtherBodyIndex :type Integer) (bFromSweep :type Boolean) (SweepResult :type Hit%20Result%20Structure%20%28by%20ref%29))
  ;[1 1 1] Get a basket
  (Utilities|IsNotPlaying
    (:true
      (bind _result (CallFunction|IsState (Variables|Default|GetPickupState) "NewEnumerator2"))
      (if (not _result)
        (bind _asbasket_bp (Utilities|Casting|CastToBasketBP OtherActor))
        (Variables|Default|SetPickupingBasket _asbasket_bp)
        (bind _result_2 (CallFunction|IsCorrectFruitsCount (Variables|Default|GetFruitsCount) (Variables|/Script/EnglishVR.Basket|GetCountItems (Variables|Default|GetPickupingBasket))))
        (if _result_2
          (Variables|Default|SetPickupState "NewEnumerator1")
          (else
            (CallFunction|PlayDialog "errors3")
            (Variables|Default|SetNegativeState "NewEnumerator1")))))))

(event OnComponentEndOverlap(PickupBox)
  (params (OverlappedComponent :type Primitive%20Component%20Object%20Reference) (OtherActor :type Actor%20Object%20Reference) (OtherComp :type Primitive%20Component%20Object%20Reference) (OtherBodyIndex :type Integer))
  ;[1 1 1] Get a basket
  (Utilities|IsNotPlaying
    (:true
      (bind _result (CallFunction|IsState (Variables|Default|GetPickupState) "NewEnumerator2"))
      (if (not _result)
        (Utilities|Casting|CastToBasketBP OtherActor)
        (Variables|Default|SetPickupState "NewEnumerator0")))))

(event Custom|OnAudioFinished_Event_AddRequest
  ;[1 1 1] Come state
  (EventDispatchers|UnbindEventfromOnAudioFinished (Variables|Default|GetAudio) (delegate Custom|OnAudioFinished_Event_AddRequest))
  (CallFunction|PlayDialog "requests4")
  (Variables|Default|SetComeState "NewEnumerator2"))

(event EventBeginPlay
  (Utilities|FlowControl|Sequence
    (:then_0
      ;[1 1 1] Dialog file select
      (Variables|Default|SetDialogTable "/Game/CSV/MainDialog.MainDialog")
      (Variables|Default|SetIsCheck true))
    (:then_1
      ;[1 1 1] Find MotionControllerPawn
      (bind _outactors (Actor|GetAllActorswithTag "MotionControllerPawn"))
      (bind _asmotion_controller_pawn (Utilities|Casting|CastToMotionControllerPawn (Utilities|Array|Get(acopy) _outactors)))
      (Variables|Default|SetPawn _asmotion_controller_pawn))
    (:then_2
      ;[1 1 1] Go to market
      (bind _arrayelement (Utilities|Array|ReverseforEachLoop (Variables|Default|GetToPath))
        (:LoopBody
          (AI|AIMoveTo (AI|GetAIController self) "0, 0, 0" _arrayelement -1.0 "Default" "Default" true true))))))

(event EventTick
  (params (DeltaSeconds :type Float%20%28single-precision%29))
  (bind _pickupingbasket (Variables|Default|GetPickupingBasket))
  (bind _mesh (Variables|/Script/EnglishVR.Basket|GetMesh _pickupingbasket))
  (Utilities|FlowControl|Sequence
    (:then_0
      (Utilities|IsNotPlaying
        (:true
          ;[1 1 1] Come state
          (bind _result (CallFunction|IsState (Variables|Default|GetComeState) "NewEnumerator1"))
          (if _result
            (CallFunction|PlayDialog "greetings4")
            (EventDispatchers|AssignOnAudioFinished (Variables|Default|GetAudio) (delegate Custom|OnAudioFinished_Event_AddRequest))))))
    (:then_1
      (Utilities|IsNotPlaying
        (:true
          ;[1 1 1] Get a basket
          (bind _result_2 (CallFunction|IsState (Variables|Default|GetPickupState) "NewEnumerator2"))
          (if (and _result_2 (not (Variables|Default|GetIsEnd)))
            (Physics|SetSimulatePhysics _mesh false)
            (Default|AttachInside _pickupingbasket)
            (Collision|SetCollisionEnabled _mesh "NoCollision")
            (Utilities|FlowControl|Delay 0.2)
            (Transformation|AttachComponentToComponent _pickupingbasket (Variables|Character|GetMesh) "RightHandSocket" "SnapToTarget" "SnapToTarget" "KeepWorld" true)
            (CallFunction|PlayDialog "goodbye3")
            (Variables|Default|SetIsEnd true)))))
    (:then_2
      (Utilities|IsNotPlaying
        (:true
          ;[1 1 1] Go away
          (if (and (Variables|Default|GetIsEnd) (not (Variables|Default|GetIsTmp)))
            (bind _arrayelement (Utilities|Array|ReverseforEachLoop (Variables|Default|GetOutPath))
              (:LoopBody
                (AI|AIMoveTo (AI|GetAIController self) "0, 0, 0" _arrayelement -1.0 "Default" "Default" true true))
              (:Completed
                (Variables|Default|SetIsTmp true)))))))))

(fn ConstructionScript)

(fn PlayDialog
  (params (DialogName :type String))
  (bind _audio (Variables|Default|GetAudio))
  (if (Variables|Default|GetIsCheck)
    (bind _returnvalue (Utilities|GetDataTableRow (Variables|Default|GetDialogTable) (Utilities|String|StringToName DialogName))
      (:then
        (bind _returnvalue_2 (Class|VictoryBPFunctionLibrary|LoadObjectfromAssetPath "/Script/Engine.SoundCue" (.Tag (Utilities|Struct|BreakRestrictedGameplayTagTableRow _returnvalue))))
        (bind _assound_cue (Utilities|Casting|CastToSoundCue _returnvalue_2)
          (:then
            (bind _output_get (Variables|Default|SetSound _assound_cue))
            (Audio|Components|Audio|SetSound _audio _output_get)
            (Audio|Components|Audio|Play _audio 0.0))
          (:CastFailed
            (Development|PrintString "Failed play sound")))))))

(fn IsState
  (params (StateA :type States%20Enum :default "NewEnumerator0") (StateB :type States%20Enum :default "NewEnumerator0"))
  (return (Utilities|Enum|Equal(Enum) StateA StateB)))

(fn IsCorrectFruitsCount
  (params (FruitsCountA :type Map%20of%20Strings%20to%20Integers) (FruitsCountB :type Map%20of%20Strings%20to%20Integers))
  (bind _keys (Utilities|Map|Keys FruitsCountA))
  (for _array_element _keys
    (if (Utilities|Map|Contains FruitsCountB _array_element)
      (if (!= (.Value (Utilities|Map|Find FruitsCountA _array_element)) (.Value (Utilities|Map|Find FruitsCountB _array_element)))
        (return false))
      (else
        (return false))))
  (return true))