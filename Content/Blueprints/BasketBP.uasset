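; A VR basket actor that a motion controller can pick up and drop, holding collectable items within its fill sphere.
; Pickup disables mesh physics and attaches the basket to the given component, while Drop re-enables physics and detaches it.
; AttachInside attaches overlapping Collectable-interface actors to the mesh and turns off collision on PickableBP items.
; DestroyInside destroys those overlapping collectables, with debug prints.
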(event EventPickup
  (params (AttachTo :type Scene%20Component%20Object%20Reference))
  (Physics|SetSimulatePhysics (Variables|Character|GetMesh) false)
  (Transformation|AttachComponentToComponent (VehicleSound|GetRootComponent) AttachTo "None" "KeepWorld" "KeepWorld" "KeepWorld" false))

(event EventDrop
  (Physics|SetSimulatePhysics (Variables|Character|GetMesh) true)
  (Transformation|DetachFromActor "KeepWorld" "KeepWorld" "KeepWorld"))

(fn ConstructionScript)

(fn DestroyInside
  (bind _fillsphere (Variables|Default|GetFillSphere))
  (bind _overlappingactors (Collision|GetOverlappingActors _fillsphere 0 :!class /Script/Engine.PrimitiveComponent))
  (for _array_element _overlappingactors
    (if (Utilities|DoesObjectImplementInterface _array_element "/Script/EnglishVR.Collectable")
      (Development|PrintString "Delete")
      (Actor|DestroyActor _array_element)))
  (Development|PrintString (Utilities|String|ToString(Integer) (Utilities|Array|Length _overlappingactors)))
  (return))

(fn AttachInside
  (for _array_element (Collision|GetOverlappingActors (Variables|Default|GetFillSphere) 0 :!class /Script/Engine.PrimitiveComponent)
    (if (Utilities|DoesObjectImplementInterface _array_element "/Script/EnglishVR.Collectable")
      (Transformation|AttachComponentToComponent (Variables|/Script/Engine.Actor|GetRootComponent _array_element) (Variables|Character|GetMesh) "None" "KeepWorld" "KeepWorld" "KeepWorld" true)
      (bind _aspickable_bp (Utilities|Casting|CastToPickableBP _array_element))
      (Collision|SetCollisionEnabled (Variables|/Game/Blueprints/PickableBP.PickableBP_C|GetStaticMeshComponent _aspickable_bp) "NoCollision"))))