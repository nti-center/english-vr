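; DestroyBoxBP is an overlap-triggered actor that removes any MyCharacter entering it, along with what that character carries.
; On overlap it copies the actors attached to the character's first attached actor into FruitArray, then destroys them.
; It then destroys that first attached actor and the character itself, and sets IsSpawned to false.
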(event Collision|EventActorBeginOverlap
  (params (OtherActor :type Actor%20Object%20Reference))
  (Utilities|Array|Clear (Variables|Default|GetFruitArray))
  (bind _asmy_character (Utilities|Casting|CastToMyCharacter OtherActor))
  (for _array_element (Actor|GetAttachedActors (Utilities|Array|Get(acopy) (Actor|GetAttachedActors _asmy_character true)) true)
    (Utilities|Array|Add (Variables|Default|GetFruitArray) _array_element))
  (for _array_element_2 (Variables|Default|GetFruitArray)
    (Actor|DestroyActor _array_element_2))
  (Actor|DestroyActor (Utilities|Array|Get(acopy) (Actor|GetAttachedActors _asmy_character true)))
  (Actor|DestroyActor _asmy_character)
  (Variables|Default|SetIsSpawned false))

(fn ConstructionScript)