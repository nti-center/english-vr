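; Test basket Blueprint that counts fruit dropped into its overlap, accepting one tagged type at a time: watermelon, then apples, then bananas.
; Overlaps matching TagArray raise FruitCount and set IsCheck; other actors get their names printed in red.
; Tick uses IsCheck to select the next tag from count thresholds.
; Tick also sets DialogCount at count milestones, but the final dialog branch is empty.
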(event Collision|EventActorBeginOverlap
  (params (OtherActor :type Actor%20Object%20Reference))
  (bind _fruitcountout (CallFunction|OnTriggerEnter OtherActor (Variables|Default|GetFruitCount) (Variables|Default|GetTagArray)))
  (if (> _fruitcountout (Variables|Default|GetFruitCount))
    (Variables|Default|SetFruitCount _fruitcountout)))

(event EventTick
  (params (DeltaSeconds :type Float%20%28single-precision%29))
  (Utilities|FlowControl|Sequence
    (:then_0
      (CallFunction|SelectTag (Variables|Default|GetFruitCount) 1 (Utilities|Array|MakeArray "Watermelon"))
      (for _array_element (Variables|Default|GetTagArray)
        _))
    (:then_1
      (CallFunction|SelectTag (Variables|Default|GetFruitCount) 7 (Utilities|Array|MakeArray "Apple")))
    (:then_2
      (CallFunction|SelectTag (Variables|Default|GetFruitCount) 13 (Utilities|Array|MakeArray "Banana")))
    (:then_3
      (if (> (Variables|Default|GetFruitCount) 0)
        (Variables|Default|SetDialogCount 1)))
    (:then_4
      (if (== (Variables|Default|GetFruitCount) 12)
        (Variables|Default|SetDialogCount 2)))
    (:then_5
      (if (== (Variables|Default|GetDialogCount) 2)
        _))))

(fn ConstructionScript)

(fn OnTriggerEnter
  (params (OtherActor :type Actor%20Object%20Reference) (FruitCount :type Integer) (OtherTagArray :type Array%20of%20Names))
  (for _array_element OtherTagArray
    (if (Actor|ActorHasTag OtherActor _array_element)
      (bind _result (Math|Integer|IncrementInt FruitCount)
        (:%20%20
          (Variables|Default|SetIsCheck true)
          (Development|PrintText "FruitCount: ")
          (Development|PrintText (Utilities|Text|ToText(Integer) _result))))
      (else
        (Development|PrintText (Utilities|Text|ToText(String) (Utilities|GetObjectName OtherActor)) true true "(R=1.000000,G=0.218681,B=0.228628,A=1.000000)" 1e+02)))
    (return _result)))

(fn SelectTag
  (params (Count :type Integer) (FructCount :type Integer) (Array :type Array%20of%20Names))
  (bind _output_get (Variables|Default|SetIsCheck (Variables|Default|GetIsCheck)))
  (if (Math|Boolean|Equal(Boolean) _output_get true)
    (if (Math|Boolean|Equal(Boolean) true (< Count FructCount))
      (for (_array_element _array_index) Array
        (Utilities|Array|SetArrayElem (Variables|Default|GetTagArray) _array_index _array_element true))
      (Variables|Default|SetIsCheck false))))