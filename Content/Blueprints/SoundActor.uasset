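; SoundActor plays sequential NPC dialogue audio, paced by the MotionControllerPawn's dialogue counter.
; BeginPlay picks among three dialogue tables using independent random rolls, so possibly none, and caches the tagged pawn.
; Once a table is set, Tick waits for the pawn's DialogCount to match its own Count, then increments it and reads that numbered row.
; The row's Tag supplies a SoundCue path, which is loaded at runtime and spawned attached to Audio.
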(event EventTick
  (params (DeltaSeconds :type Float%20%28single-precision%29))
  ;[1 1 1] Play NPC dialogue
  (if (Math|Boolean|Equal(Boolean) (Variables|Default|GetCheck) true)
    (if (== (Variables|/Game/VirtualRealityBP/Blueprints/MotionControllerPawn.MotionControllerPawn_C|GetDialogCount (Variables|Default|GetPawn)) (Variables|Default|GetCount))
      (bind _output_get (Variables|Default|SetCount (Variables|Default|GetCount)))
      (bind _result (Math|Integer|IncrementInt _output_get)
        (:%20%20
          (bind _output_get_2 (Variables|Default|SetCount _result))
          (bind _returnvalue (Utilities|GetDataTableRow (Variables|Default|GetDialogTable) (Utilities|String|StringToName (Utilities|String|ToString(Text) (Utilities|Text|ToText(Integer) _output_get_2))))
            (:then
              (bind _returnvalue_2 (Class|VictoryBPFunctionLibrary|LoadObjectfromAssetPath "/Script/Engine.SoundCue" (.Tag (Utilities|Struct|BreakRestrictedGameplayTagTableRow _returnvalue))))
              (bind _assound_cue (Utilities|Casting|CastToSoundCue _returnvalue_2)
                (:then
                  (bind _output_get_3 (Variables|Default|SetSound _assound_cue))
                  (Audio|SpawnSoundAttached _output_get_3 (Variables|Default|GetAudio) "None" "0, 0, 0" "0, 0, 0" "KeepRelativeOffset" false 1.0 1.0 0.0 0 0))
                (:CastFailed
                  (Development|PrintString "Failed"))))))))))

(event EventBeginPlay
  (bind _returnvalue (Math|Random|RandomInteger 3))
  (Utilities|FlowControl|Sequence
    (:then_0
      ;[1 1 1] Dialog file select
      (Utilities|FlowControl|Sequence
        (:then_0
          (if (== 0 _returnvalue)
            (bind _output_get (Variables|Default|SetTable1 "/Game/CSV/PathToDialog.PathToDialog"))
            (Variables|Default|SetDialogTable _output_get)
            (Variables|Default|SetCheck true :!label _label)))
        (:then_1
          (if (== 1 _returnvalue)
            (bind _output_get_2 (Variables|Default|SetTable2 "/Game/CSV/PathToDialog.PathToDialog"))
            (Variables|Default|SetDialogTable _output_get_2)
            (goto _label)))
        (:then_2
          (if (== 2 _returnvalue)
            (bind _output_get_3 (Variables|Default|SetTable3 "/Game/CSV/PathToDialog.PathToDialog"))
            (Variables|Default|SetDialogTable _output_get_3)
            (goto _label)))))
    (:then_1
      ;[1 1 1] Find MotionControllerPawn
      (bind _outactors (Actor|GetAllActorswithTag "MotionControllerPawn"))
      (bind _asmotion_controller_pawn (Utilities|Casting|CastToMotionControllerPawn (Utilities|Array|Get(acopy) _outactors)))
      (Variables|Default|SetPawn _asmotion_controller_pawn))))

(fn ConstructionScript)