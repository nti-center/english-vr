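; Hotel door Blueprint with a physics-driven door that eases back to a zero rotation after being hit.
; A component hit stops any running timeline and, after a two-second delay, plays it from the start.
; Each timeline update lerps from the current world rotation toward zero, applies it as relative rotation, and toggles physics simulation off and on.
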(event OnComponentHit(Door)
  (params (HitComponent :type Primitive%20Component%20Object%20Reference) (OtherActor :type Actor%20Object%20Reference) (OtherComp :type Primitive%20Component%20Object%20Reference) (NormalImpulse :type Vector :default "0, 0, 0") (Hit :type Hit%20Result%20Structure%20%28by%20ref%29))
  (Utilities|FlowControl|Sequence
    (:then_0
      (Utilities|FlowControl|Delay 2.0)
      (bind _driver (Timeline|Timeline_0 PlayFromStart)
        (:Update
          (Transformation|SetRelativeRotation (Variables|Default|GetDoor) (Math|Rotator|Lerp(Rotator) (Transformation|GetWorldRotation (Variables|Default|GetDoor)) "0, 0, 0" _driver) false false)
          (Physics|SetSimulatePhysics (Variables|Default|GetDoor) false)
          (Physics|SetSimulatePhysics (Variables|Default|GetDoor) true))))
    (:then_1
      (Timeline|Timeline_0 Stop))))

(event EventBeginPlay)

(event Collision|EventActorBeginOverlap
  (params (OtherActor :type Actor%20Object%20Reference)))

(event EventTick
  (params (DeltaSeconds :type Float%20%28single-precision%29)))

(fn ConstructionScript)